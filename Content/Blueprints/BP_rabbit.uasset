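; Bonnie rabbit animatronic enemy for a FNAF-style night game, advancing through attack phases toward the player.
; A looping timer rolls BonnieLevel against a random number to advance Phase, but only when the night manager's GameOver or NightComplete is true.
; At the third phase, a delayed sound precedes a player DoorClosed check that resets Bonnie or starts the attack.
; Tick applies each phase's position and animation, then spawns a chase actor once and flags Jumpscare.
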(event `BonnieLogic`
  (`KismetSystemLibrary.PrintString` "bonnie logic")
  (bind _asgmb_night_manager (cast `/Game/Blueprints/GMB_NightManager` (`GameplayStatics.GetGameMode`)))
  (if (or (== (`/Game/Blueprints/GMB_NightManager.GameOver` _asgmb_night_manager) true) (== (`/Game/Blueprints/GMB_NightManager.NightComplete` _asgmb_night_manager) true))
    (set `self.RandomNumber` (`KismetMathLibrary.RandomIntegerInRange` 0 20))
    (if (>= (`self.BonnieLevel`) (`self.RandomNumber`))
      (if (== (`self.Phase`) 3)
        (`KismetSystemLibrary.Delay` 15.5)
        (`GameplayStatics.PlaySoundAtLocation` null (0.0 0.0 0.0) (struct) 1.0 1.0 0.0 null null null null)
        (`KismetSystemLibrary.PrintString` "close the door")
        (`KismetSystemLibrary.Delay` 4.5)
        (bind _returnvalue (`GameplayStatics.GetActorOfClass` "/Game/FirstPerson/Blueprints/BP_FirstPersonCharacter.BP_FirstPersonCharacter_C"))
        (if (`/Game/FirstPerson/Blueprints/BP_FirstPersonCharacter.DoorClosed?` _returnvalue)
          (set `self.Phase` 0)
          (`KismetSystemLibrary.PrintString` "bonnie reset")
          (else
            (set `self.Phase` 4)))
        (else
          (set `self.Phase` (+ (`self.Phase`) 1))
          (`KismetSystemLibrary.PrintString` (`KismetStringLibrary.Conv_IntToString` (`self.Phase`)))))
      (else
        (`KismetSystemLibrary.PrintString` "bonnie rolled false")))
    (else
      (`KismetSystemLibrary.PrintString` "bonnie false"))))

(event `self.ReceiveBeginPlay`
  (`KismetSystemLibrary.PrintString` "Levelstart(bonnie)")
  (`KismetSystemLibrary.K2_SetTimerDelegate` (delegate `BonnieLogic`) 3.0 true true))

(event `self.ReceiveTick`
  (params (DeltaSeconds :type "Float (single-precision)"))
  (switch `int` (`self.Phase`)
    (:`1`
      (`self.K2_SetActorLocation` (`self.Phase1Vector`))
      (`SkeletalMeshComponent.PlayAnimation` (`self.Mesh`) "/Game/MAP/ignited_bonnie/SkeletalMeshes/ignited_bonnieWithered_Bonnie_Withered_Bonnie_Withered_Bonnie--Glimpse.ignited_bonnieWithered_Bonnie_Withered_Bonnie_Withered_Bonnie--Glimpse" false))
    (:`2`
      (`self.K2_SetActorLocation` (`self.Phase2Vector`))
      (`SkeletalMeshComponent.PlayAnimation` (`self.Mesh`) "/Game/MAP/ignited_bonnie/SkeletalMeshes/ignited_bonnieWithered_Bonnie_Withered_Bonnie_Withered_Bonnie--Glimpse_2_.ignited_bonnieWithered_Bonnie_Withered_Bonnie_Withered_Bonnie--Glimpse_2_" false))
    (:`3`
      (`self.K2_SetActorLocation` (`self.Phase3Vector`))
      (`SkeletalMeshComponent.PlayAnimation` (`self.Mesh`) "/Game/MAP/ignited_bonnie/SkeletalMeshes/ignited_bonnieWithered_Bonnie_Withered_Bonnie_Withered_Bonnie--Shutdown.ignited_bonnieWithered_Bonnie_Withered_Bonnie_Withered_Bonnie--Shutdown" false))
    (:`4`
      (if (not (`self.Spawned`))
        (`|SpawnActorFromClass` "/Game/Blueprints/BP_RabbitChase.BP_RabbitChase_C" (`self.ChaseTransform`) "Undefined" "MultiplyWithRoot" null null)
        (set `self.Spawned` true)
        (set `self.Jumpscare` true)))))

(fn `UserConstructionScript`)