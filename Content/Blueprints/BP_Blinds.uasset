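; BP_Blinds is a trigger actor that sets a flag on the first-person player character while the player is inside its Box.
; On begin overlap, it sets PlayerCock2 to true on BP_FirstPersonCharacter if the overlapping actor is the player.
; On end overlap, it clears the flag without checking which actor left.
; Both events print debug strings, and the file contains no blind movement logic.
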(event `self.Box.OnComponentBeginOverlap`
  (params (OverlappedComponent :type "PrimitiveComponent Object Reference") (OtherActor :type "Actor Object Reference") (OtherComp :type "PrimitiveComponent Object Reference") (OtherBodyIndex :type Integer) (bFromSweep :type Boolean) (SweepResult :type "HitResult Structure (by ref)"))
  (bind _asbp_first_person_character (cast `/Game/FirstPerson/Blueprints/BP_FirstPersonCharacter` (`GameplayStatics.GetPlayerCharacter` 0)))
  (bind _output_get (set `self.As BP First Person Character` _asbp_first_person_character))
  (if (== OtherActor (`GameplayStatics.GetPlayerCharacter` 0))
    (set `/Game/FirstPerson/Blueprints/BP_FirstPersonCharacter.PlayerCock2` true _output_get)
    (`KismetSystemLibrary.PrintString` "sus")))

(event `self.Box.OnComponentEndOverlap`
  (params (OverlappedComponent :type "PrimitiveComponent Object Reference") (OtherActor :type "Actor Object Reference") (OtherComp :type "PrimitiveComponent Object Reference") (OtherBodyIndex :type Integer))
  (bind _asbp_first_person_character (cast `/Game/FirstPerson/Blueprints/BP_FirstPersonCharacter` (`GameplayStatics.GetPlayerCharacter` 0)))
  (set `/Game/FirstPerson/Blueprints/BP_FirstPersonCharacter.PlayerCock2` false _asbp_first_person_character)
  (`KismetSystemLibrary.PrintString` "asd"))

(fn `UserConstructionScript`)