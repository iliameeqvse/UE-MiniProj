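; GMB_NightManager runs the night clock, apparently as a game mode, tracking the current hour and whether the night ends in completion or game over.
; A looping timer started on BeginPlay increments the hour every SecondsPerHour.
; TriggerNightComplete and GameOverTrigger each set their flag and clear that timer.
; The six-hour check is unconnected and the branch is always true, so the first tick completes the night.
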(event `TriggerNightComplete`
  (set `self.NightComplete` true)
  (`KismetSystemLibrary.K2_ClearAndInvalidateTimerHandle` (`self.HourTimerHandle`)))

(event `AdvanceHour`
  (`/Engine/EditorBlueprintResources/StandardMacros.IncrementInt` (`self.CurrentHour`)
    (:`  `
      (if true
        (`self.TriggerNightComplete`)))))

(event `self.ReceiveBeginPlay`
  (bind _returnvalue (`KismetSystemLibrary.K2_SetTimerDelegate` (delegate `AdvanceHour`) (`self.SecondsPerHour`) true))
  (set `self.HourTimerHandle` _returnvalue))

(event `GameOverTrigger`
  (set `self.GameOver` true)
  (`KismetSystemLibrary.K2_ClearAndInvalidateTimerHandle` (`self.HourTimerHandle`)))

(fn `UserConstructionScript`)